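; Enemy Blueprint that heads for the nearest turret and attacks it, with a camera-facing health bar.
; Tick refreshes the bar and re-issues the move until within range, which sets IsAttacking.
; AttackBox overlap with a turret stops movement and starts a looping damage timer.
; Damage lowers Health, notifying Spawner and destroying the enemy at exactly zero, otherwise moving toward the instigator; older player-detection chase logic is disconnected.
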(event OnComponentBeginOverlap(AttackBox)
  (params (OverlappedComponent :type Primitive%20Component%20Object%20Reference) (OtherActor :type Actor%20Object%20Reference) (OtherComp :type Primitive%20Component%20Object%20Reference) (OtherBodyIndex :type Integer) (bFromSweep :type Boolean) (SweepResult :type Hit%20Result%20Structure%20%28by%20ref%29))
  ;[0.1562 0.1562 0.1562] Si la tour est dans son champ d'attaque, attaque
  (if (Class|GameplayStatics|ObjectIsA OtherActor "/Game/Blueprints/BP_Turret.BP_Turret_C")
    (Pawn|Components|CharacterMovement|DisableMovement (Variables|Character|GetCharacterMovement))
    (Variables|Default|SetIsAttacking true)
    (Utilities|Time|SetTimerbyEvent (delegate Custom|Attack) 1.0 true)))

(event OnComponentEndOverlap(AttackBox)
  (params (OverlappedComponent :type Primitive%20Component%20Object%20Reference) (OtherActor :type Actor%20Object%20Reference) (OtherComp :type Primitive%20Component%20Object%20Reference) (OtherBodyIndex :type Integer))
  ;[0.1562 0.1562 0.1562] Si le joueur quitte son champ d'attaque, le poursuivre (si c'est la tour qu'il attaque, cette node ne sera jamais appelée) [désactivée]
)

(event OnComponentBeginOverlap(DetectionBox)
  (params (OverlappedComponent :type Primitive%20Component%20Object%20Reference) (OtherActor :type Actor%20Object%20Reference) (OtherComp :type Primitive%20Component%20Object%20Reference) (OtherBodyIndex :type Integer) (bFromSweep :type Boolean) (SweepResult :type Hit%20Result%20Structure%20%28by%20ref%29))
  ;[0.1562 0.1562 0.1562] Détection du joueur (désactivé)
)

(event Custom|Attack
  ;[0.1562 0.1562 0.1562] Si la tour est dans son champ d'attaque, attaque
  (Game|Damage|ApplyDamage (stale OnComponentBeginOverlap(AttackBox) OtherActor) 1.0 (Pawn|GetController) self))

(event EventBeginPlay
  ;[0.1562 0.1562 0.1562] Se dirige vers la tour la plus proche dès son apparition (ancien code)
  (Variables|Default|SetMaxHealth (Variables|Default|GetHealth)))

(event EventTick
  (params (DeltaSeconds :type Float%20%28single-precision%29))
  (bind _returnvalue (Transformation|GetActorLocation))
  (bind _health_bar_widget (Variables|Default|GetHealth%20Bar%20Widget))
  (bind _turrets (Variables|Default|GetTurrets))
  (bind (_distance _returnvalue_2) (Actor|FindNearestActor _returnvalue _turrets))
  ;[0.1562 0.1562 0.1562] Se dirige en continue vers la tour la plus proche dès son apparition
  ;[1 0.3385 0.3385] Enemy healthbar system
  (Utilities|FlowControl|Sequence
    (:then_0
      (bind _aswb_health_bar (Utilities|Casting|CastToWB_HealthBar (UserInterface|GetWidget (Variables|Default|GetHealth%20Bar%20Widget))))
      (Progress|SetPercent (Variables|/Game/Blueprints/UI/WB_HealthBar.WB_HealthBar_C|GetHealthBar _aswb_health_bar) (/ (/ (* (Variables|Default|GetHealth) 100) (Variables|Default|GetMaxHealth)) 1e+02))
      (Transformation|SetWorldRotation _health_bar_widget (Math|Rotator|FindLookatRotation (Transformation|GetWorldLocation _health_bar_widget) (Transformation|GetWorldLocation (Variables|/Script/Engine.PlayerCameraManager|GetTransformComponent (Game|GetPlayerCameraManager 0)))) false false))
    (:then_1
      (if (!= (Variables|Default|GetIsAttacking) true)
        (Variables|Default|SetTarget _returnvalue_2)
        (AI|Navigation|SimpleMovetoActor (AI|GetAIController self) _returnvalue_2)
        (if (< _distance 2e+02)
          (Variables|Default|SetIsAttacking true))))))

(event Game|Damage|EventAnyDamage
  (params (Damage :type Float%20%28single-precision%29) (DamageType :type Damage%20Type%20Object%20Reference) (InstigatedBy :type Controller%20Object%20Reference) (DamageCauser :type Actor%20Object%20Reference))
  ;[1 1 1] Apply Damage - Chase Player on Damage
  (Development|PrintString "Enemy hurt")
  (bind _output_get (Variables|Default|SetHealth (- (Variables|Default|GetHealth) Damage)))
  (Development|PrintString (Utilities|String|ToString(Integer) (Math|Float|Truncate _output_get)))
  (if (== _output_get 0)
    (Default|RemoveEnemy (Variables|Default|GetSpawner))
    (Actor|DestroyActor)
    (else
      (AI|Navigation|SimpleMovetoActor (AI|GetAIController self) InstigatedBy))))

(fn ConstructionScript)