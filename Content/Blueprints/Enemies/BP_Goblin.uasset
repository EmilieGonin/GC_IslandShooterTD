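; Goblin enemy that heads for the BP_Turret on spawn and switches to hunting the player once detected.
; A detection box overlap halts it briefly while Tick turns its capsule toward the player, then AIMoveTo starts the chase.
; An attack box overlap with turret or player stops movement and sets IsAttacking; any end overlap clears it and resumes pursuit of the player.
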(event OnComponentBeginOverlap(AttackBox)
  (params (OverlappedComponent :type Primitive%20Component%20Object%20Reference) (OtherActor :type Actor%20Object%20Reference) (OtherComp :type Primitive%20Component%20Object%20Reference) (OtherBodyIndex :type Integer) (bFromSweep :type Boolean) (SweepResult :type Hit%20Result%20Structure%20%28by%20ref%29))
  ;[0.1562 0.1562 0.1562] Si l'acteur est le joueur ou la tour sont dans son champ d'attaque, attaque
  (bind _returnvalue (Actor|GetActorOfClass "/Game/Blueprints/BP_Turret.BP_Turret_C"))
  (if (or (== _returnvalue OtherActor) (== OtherActor (Game|Player|GetPlayerPawn 0)))
    (Pawn|Components|CharacterMovement|DisableMovement (Variables|Character|GetCharacterMovement))
    (Variables|Default|SetIsAttacking true)))

(event OnComponentEndOverlap(AttackBox)
  (params (OverlappedComponent :type Primitive%20Component%20Object%20Reference) (OtherActor :type Actor%20Object%20Reference) (OtherComp :type Primitive%20Component%20Object%20Reference) (OtherBodyIndex :type Integer))
  ;[0.1562 0.1562 0.1562] Si le joueur quitte son champ d'attaque, le poursuivre (si c'est la tour qu'il attaque, cette node ne sera jamais appelée)
  (Variables|Default|SetIsAttacking false)
  (Pawn|Components|CharacterMovement|SetMovementMode (Variables|Character|GetCharacterMovement) "MOVE_NavWalking" 0)
  (AI|AIMoveTo self "0, 0, 0" (Game|Player|GetPlayerPawn 0) 5.0 false))

(event OnComponentBeginOverlap(DetectionBox)
  (params (OverlappedComponent :type Primitive%20Component%20Object%20Reference) (OtherActor :type Actor%20Object%20Reference) (OtherComp :type Primitive%20Component%20Object%20Reference) (OtherBodyIndex :type Integer) (bFromSweep :type Boolean) (SweepResult :type Hit%20Result%20Structure%20%28by%20ref%29))
  ;[0.1562 0.1562 0.1562] Détection du joueur
  (if (and (and (== OtherActor (Game|Player|GetPlayerPawn 0)) (not (Variables|Default|GetStartChasing))) (not (Variables|Default|GetIsAttacking)))
    (Variables|Default|SetSawPlayer true)
    (Pawn|Components|CharacterMovement|DisableMovement (Variables|Character|GetCharacterMovement))
    (Utilities|FlowControl|Delay 0.8)
    (Variables|Default|SetSawPlayer false)
    (Variables|Default|SetStartChasing true)
    (Pawn|Components|CharacterMovement|SetMovementMode (Variables|Character|GetCharacterMovement) "MOVE_NavWalking" 0)
    (AI|AIMoveTo self "0, 0, 0" (Game|Player|GetPlayerPawn 0) 5.0 false)))

(event EventBeginPlay
  ;[0.1562 0.1562 0.1562] Se dirige vers la tour dès son apparition
  (bind _returnvalue (Actor|GetActorOfClass "/Game/Blueprints/BP_Turret.BP_Turret_C"))
  (AI|AIMoveTo self "0, 0, 0" _returnvalue 5.0 false))

(event EventTick
  (params (DeltaSeconds :type Float%20%28single-precision%29))
  ;[0.1562 0.1562 0.1562] Si le joueur a été aperçu, le regarde jusqu'à ce qu'il commence à le chasser
  (if (Variables|Default|GetSawPlayer)
    (Transformation|SetWorldRotation (Variables|Default|GetCapsuleComponent) (Math|Rotator|MakeRotfromX (Math|Vector|Normalize (- (Transformation|GetActorLocation (Game|Player|GetPlayerPawn 0)) (Transformation|GetActorLocation)))) false false)))

(fn ConstructionScript
  (|CallParentFunction))