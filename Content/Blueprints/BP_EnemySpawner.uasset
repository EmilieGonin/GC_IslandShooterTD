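; BP_EnemySpawner is an actor that periodically spawns BP_Lich enemies at its own location.
; A Delay on Tick paces the cycle at roughly four seconds, incrementing EnemyNumber each time.
; Spawning is skipped only when the count equals ten, so it resumes afterwards rather than stopping.
; A random three-way switch picks a branch, but all branches spawn the same class and print debug strings.
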(event EventBeginPlay)

(event Collision|EventActorBeginOverlap
  (params (OtherActor :type Actor%20Object%20Reference)))

(event EventTick
  (params (DeltaSeconds :type Float%20%28single-precision%29))
  (bind _returnvalue (Math|Random|RandomIntegerinRange 0 2))
  (bind _returnvalue_2 (Transformation|GetActorLocation))
  (bind _returnvalue_3 (Utilities|String|ToString(Integer) _returnvalue))
  (bind _returnvalue_4 (Math|Conversions|ToTransform(Vector) _returnvalue_2))
  (Utilities|FlowControl|Delay 4.0)
  (Variables|Default|SetEnemyNumber (+ (Variables|Default|GetEnemyNumber) 1))
  (if (!= (Variables|Default|GetEnemyNumber) 10)
    (switch int _returnvalue
      (:0
        (Development|PrintString _returnvalue_3)
        (Game|SpawnActorfromClass "/Game/Blueprints/BP_Lich.BP_Lich_C" _returnvalue_4 "Undefined" "MultiplyWithRoot" 0 0))
      (:1
        (Development|PrintString _returnvalue_3)
        (Game|SpawnActorfromClass "/Game/Blueprints/BP_Lich.BP_Lich_C" _returnvalue_4 "Undefined" "MultiplyWithRoot" 0 0))
      (:2
        (Development|PrintString _returnvalue_3)
        (Game|SpawnActorfromClass "/Game/Blueprints/BP_Lich.BP_Lich_C" _returnvalue_4 "Undefined" "MultiplyWithRoot" 0 0)))
    (Development|PrintString "New enemy spawned")))

(fn ConstructionScript)