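; BP_NewBullet is a projectile Blueprint that damages enemies it collides with.
; Its Sphere hit event acts only on BP_Enemy actors, applying a fixed amount of damage credited to the first player controller, then destroying the bullet.
; Hits on other actors are ignored, leaving the bullet in place.
; Debug prints mark the hit, and a trailing Character cast has no meaningful effect.
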(event OnComponentHit(Sphere)
  (params (HitComponent :type Primitive%20Component%20Object%20Reference) (OtherActor :type Actor%20Object%20Reference) (OtherComp :type Primitive%20Component%20Object%20Reference) (NormalImpulse :type Vector :default "0, 0, 0") (Hit :type Hit%20Result%20Structure%20%28by%20ref%29))
  ;[0.05035 0.05035 0.05035] Check if an enemy is hit
  (if (Class|GameplayStatics|ObjectIsA OtherActor "/Game/Blueprints/Enemies/BP_Enemy.BP_Enemy_C")
    (Development|PrintString "Event Hit")
    ;[1 1 1] Apply Damage if target is an enemy
    (Utilities|FlowControl|Sequence
      (:then_0
        (if true
          (Development|PrintString "Enemy Hit")
          (Game|Damage|ApplyDamage OtherActor 1.0 (Game|GetPlayerController 0) self)
          (bind _ascharacter (Utilities|Casting|CastToCharacter OtherActor))
          (Variables|Default|SetTarget _ascharacter)))
      (:then_1
        (Actor|DestroyActor) ; Then destroy this projectile
      ))))

(fn ConstructionScript)