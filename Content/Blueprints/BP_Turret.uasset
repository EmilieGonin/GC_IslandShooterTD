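; Turret that fires physics-driven bullets at an enemy in range and can take damage.
; After a startup delay, a looping timer gets a single BP_Enemy (not necessarily the nearest), checks range, then spawns a Bullet above itself and impulses its sphere toward that enemy.
; Damage lowers Life, destroying the turret only at exactly zero, otherwise ordering an AI move toward the instigator.
; Destruction calls OnTurretDestroy.
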(event Custom|Fire
  ;[1 1 1] Check for enemy in range
  (bind _returnvalue (Actor|GetActorOfClass "/Game/Blueprints/Enemies/BP_Enemy.BP_Enemy_C"))
  (Variables|Default|SetEnemy _returnvalue)
  (if (< (Transformation|GetDistanceTo (Variables|Default|GetEnemy)) (Variables|Default|GetRange))
    (bind _returnvalue_2 (Game|SpawnActorfromClass (Variables|Default|GetBullet) (Math|Conversions|ToTransform(Vector) (+ (Transformation|GetActorLocation) "0.000000,0.000000,250.000000")) "Undefined" "MultiplyWithRoot" 0 0))
    ;[1 1 1] Fire Bullet created from precedent node
    (Utilities|IsValid (Variables|/Game/Blueprints/Bullets/BP_NewBullet.BP_NewBullet_C|GetSphere _returnvalue_2)
      (:Is%20Valid
        (Physics|AddImpulseatLocation (Variables|/Game/Blueprints/Bullets/BP_NewBullet.BP_NewBullet_C|GetSphere _returnvalue_2) (* (Math|Vector|GetUnitDirection(Vector) (Transformation|GetWorldLocation (Variables|/Script/Engine.Actor|GetRootComponent _returnvalue_2)) (Transformation|GetActorLocation (Variables|Default|GetEnemy))) (Variables|Default|GetBullet_Speed)) (Transformation|GetActorLocation (Variables|Default|GetEnemy)) "None")))))

(event EventBeginPlay
  ;[1 1 1] Set Fire Rate Of the turret
  (Utilities|FlowControl|Delay 5.0)
  (Utilities|Time|SetTimerbyEvent (delegate Custom|Fire) (Variables|Default|GetFire%20Rate) true))

(event EventDestroyed
  ;[1 1 1] Call for Destroyed Turret
  (Development|PrintString "Turret destroued")
  (Default|CallOnTurretDestroy))

(event Game|Damage|EventAnyDamage
  (params (Damage :type Float%20%28single-precision%29) (DamageType :type Damage%20Type%20Object%20Reference) (InstigatedBy :type Controller%20Object%20Reference) (DamageCauser :type Actor%20Object%20Reference))
  ;[1 1 1] Apply Damage - Chase Player on Damage
  (Development|PrintString "Turret hurt")
  (bind _output_get (Variables|Default|SetLife (- (Variables|Default|GetLife) Damage)))
  (if (== _output_get 0.0)
    (Actor|DestroyActor)
    (else
      (AI|Navigation|SimpleMovetoActor (AI|GetAIController self) InstigatedBy))))

(fn ConstructionScript)